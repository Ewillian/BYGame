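; Game instance that exposes events for showing the main menu, options, gauge HUD and tutorial widgets.
; Each event adds its widget to the viewport and turns on the mouse cursor.
; The main and option menu events share one cached W_MainMenu, so both show the same widget, while the HUD and tutorial widgets are created anew on each call.
; An unconnected language selection block repeats the main menu logic.
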(event EventShowMainMenu
  ;[1 1 1] Show Main Menu
  (Variables|Default|Getw_mainMenu
    (:then
      _)
    (:else
      (bind _returnvalue (UserInterface|CreateWidget "/Game/MainMenu/W_MainMenu.W_MainMenu_C" (Game|GetPlayerController 0)))
      (bind _output_get (Variables|Default|Setw_mainMenu _returnvalue))))
  (UserInterface|Viewport|AddtoViewport _output_get 0)
  (Variables|/Script/Engine.PlayerController|SetbShowMouseCursor (Game|GetPlayerController 0) true))

(event EventShowTutorial
  (bind _returnvalue (UserInterface|CreateWidget "/Game/GameComponents/Widget/W_Tutorial.W_Tutorial_C" (Game|GetPlayerController 0)))
  (bind _output_get (Variables|Default|Setw_tutorial _returnvalue))
  (UserInterface|Viewport|AddtoViewport _output_get 0)
  (Variables|/Script/Engine.PlayerController|SetbShowMouseCursor (Game|GetPlayerController 0) true))

(event EventShowGameInterface
  ;[1 1 1] Show Main Menu
  (bind _returnvalue (UserInterface|CreateWidget "/Game/GameComponents/Widget/W_UserJauge.W_UserJauge_C" (Game|GetPlayerController 0)))
  (bind _output_get (Variables|Default|Setw_userJauge _returnvalue))
  (UserInterface|Viewport|AddtoViewport _output_get 0)
  (Variables|/Script/Engine.PlayerController|SetbShowMouseCursor (Game|GetPlayerController 0) true))

(event EventShowOptionMenu
  ;[1 1 1] Show Option Menu
  (Variables|Default|Getw_mainMenu
    (:then
      _)
    (:else
      (bind _returnvalue (UserInterface|CreateWidget "/Game/MainMenu/W_MainMenu.W_MainMenu_C" (Game|GetPlayerController 0)))
      (bind _output_get (Variables|Default|Setw_mainMenu _returnvalue))))
  (UserInterface|Viewport|AddtoViewport _output_get 0)
  (Variables|/Script/Engine.PlayerController|SetbShowMouseCursor (Game|GetPlayerController 0) true))